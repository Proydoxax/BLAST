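; Tutorial manager actor that walks the player through the rhythm game's controls: moving, hitting a note, holding and releasing a slider, then an HP, combo and points overview.
; BeginPlay creates WBP_Tutorial and freezes play with near-zero time dilation while pausing the song on BP_NoteSpawner.
; Tick runs a step state machine, polling character input flags to resume, then re-freezing after hand-tuned delays at the next prompt.
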(event `self.ReceiveBeginPlay`
  (bind _outactors (`GameplayStatics.GetAllActorsOfClass` "/Game/Game/Notes/NoteHandler/BP_NoteSpawner.BP_NoteSpawner_C"))
  (set `self.NoteSpawnerRef ` (`|GetArrayItem` _outactors))
  (bind _asthird_person_character (cast `/Game/Game/Character/Blueprints/ThirdPersonCharacter` (`GameplayStatics.GetPlayerCharacter` 0)))
  (set `self.CharacterRef` _asthird_person_character)
  (bind _returnvalue (`|CreateWidget` "/Game/UI/Widgets/WBP_Tutorial.WBP_Tutorial_C" (`GameplayStatics.GetPlayerController` 0)))
  (set `self.TutorialWidget` _returnvalue)
  (`UserWidget.AddToViewport` (`self.TutorialWidget`) 0)
  (set `self.CurrentStep` 0)
  (set `self.bTutorialPaused` true)
  (`KismetSystemLibrary.Delay` 0.5)
  (`GameplayStatics.SetGlobalTimeDilation` 0.001)
  (`/Game/Game/Notes/NoteHandler/BP_NoteSpawner.PauseSongGameplay` (`self.NoteSpawnerRef `)))

(event `self.ReceiveTick`
  (params (DeltaSeconds :type "Float (single-precision)"))
  (switch `int` (`self.CurrentStep`)
    (:`0`
      (`TextBlock.SetText` (`/Game/UI/Widgets/WBP_Tutorial.TXT_Tutorial` (`self.TutorialWidget`)) "Use A and D to move")
      (if (`/Game/Game/Character/Blueprints/ThirdPersonCharacter.bMoved` (`self.CharacterRef`))
        (`GameplayStatics.SetGlobalTimeDilation` 1.0)
        (`/Game/Game/Notes/NoteHandler/BP_NoteSpawner.ResumeSongGameplay` (`self.NoteSpawnerRef `))
        (set `self.CurrentStep` 1)
        (`Widget.SetVisibility` (`self.TutorialWidget`) "Hidden")
        (`KismetSystemLibrary.Delay` 2.1)
        (`Widget.SetVisibility` (`self.TutorialWidget`) "Visible")
        (`GameplayStatics.SetGlobalTimeDilation` 0.001)
        (`/Game/Game/Notes/NoteHandler/BP_NoteSpawner.PauseSongGameplay` (`self.NoteSpawnerRef `))))
    (:`1`
      (`TextBlock.SetText` (`/Game/UI/Widgets/WBP_Tutorial.TXT_Tutorial` (`self.TutorialWidget`)) "Press SPACE to hit the note")
      (if (`/Game/Game/Character/Blueprints/ThirdPersonCharacter.bHitNote` (`self.CharacterRef`))
        (`GameplayStatics.SetGlobalTimeDilation` 1.0)
        (`/Game/Game/Notes/NoteHandler/BP_NoteSpawner.ResumeSongGameplay` (`self.NoteSpawnerRef `))
        (set `self.CurrentStep` 2)
        (`Widget.SetVisibility` (`self.TutorialWidget`) "Hidden")
        (`KismetSystemLibrary.Delay` 9.1)
        (`Widget.SetVisibility` (`self.TutorialWidget`) "Visible")
        (`GameplayStatics.SetGlobalTimeDilation` 0.001)
        (`/Game/Game/Notes/NoteHandler/BP_NoteSpawner.PauseSongGameplay` (`self.NoteSpawnerRef `))))
    (:`2`
      (`TextBlock.SetText` (`/Game/UI/Widgets/WBP_Tutorial.TXT_Tutorial` (`self.TutorialWidget`)) "Hold SPACE to begin the slider")
      (if (`/Game/Game/Character/Blueprints/ThirdPersonCharacter.isHoldingSpace` (`self.CharacterRef`))
        (`GameplayStatics.SetGlobalTimeDilation` 1.0)
        (`/Game/Game/Notes/NoteHandler/BP_NoteSpawner.ResumeSongGameplay` (`self.NoteSpawnerRef `))
        (set `self.CurrentStep` 3)
        (`Widget.SetVisibility` (`self.TutorialWidget`) "Hidden")
        (`KismetSystemLibrary.Delay` 1.8)
        (`Widget.SetVisibility` (`self.TutorialWidget`) "Visible")
        (`GameplayStatics.SetGlobalTimeDilation` 0.001)
        (`/Game/Game/Notes/NoteHandler/BP_NoteSpawner.PauseSongGameplay` (`self.NoteSpawnerRef `))))
    (:`3`
      (`TextBlock.SetText` (`/Game/UI/Widgets/WBP_Tutorial.TXT_Tutorial` (`self.TutorialWidget`)) "Release SPACE to complete the slider")
      (if (not (`/Game/Game/Character/Blueprints/ThirdPersonCharacter.isHoldingSpace` (`self.CharacterRef`)))
        (`GameplayStatics.SetGlobalTimeDilation` 1.0)
        (`/Game/Game/Notes/NoteHandler/BP_NoteSpawner.ResumeSongGameplay` (`self.NoteSpawnerRef `))
        (set `self.CurrentStep` 4)
        (`Widget.SetVisibility` (`self.TutorialWidget`) "Hidden")
        (`KismetSystemLibrary.Delay` 7.0)
        (`Widget.SetVisibility` (`self.TutorialWidget`) "Visible")
        (`Widget.SetVisibility` (`/Game/UI/Widgets/WBP_Tutorial.HP_text` (`self.TutorialWidget`)) "Visible")
        (`Widget.SetVisibility` (`/Game/UI/Widgets/WBP_Tutorial.combo_Text` (`self.TutorialWidget`)) "Visible")
        (`Widget.SetVisibility` (`/Game/UI/Widgets/WBP_Tutorial.points_Text` (`self.TutorialWidget`)) "Visible")
        (`Widget.SetVisibility` (`/Game/UI/Widgets/WBP_Tutorial.continue_Text` (`self.TutorialWidget`)) "Visible")
        (`Widget.SetVisibility` (`/Game/UI/Widgets/WBP_Tutorial.TXT_Tutorial` (`self.TutorialWidget`)) "Hidden")
        (`GameplayStatics.SetGlobalTimeDilation` 0.001)
        (`/Game/Game/Notes/NoteHandler/BP_NoteSpawner.PauseSongGameplay` (`self.NoteSpawnerRef `))))
    (:`4`
      (if (`/Game/Game/Character/Blueprints/ThirdPersonCharacter.bContinue` (`self.CharacterRef`))
        (`GameplayStatics.SetGlobalTimeDilation` 1.0)
        (`/Game/Game/Notes/NoteHandler/BP_NoteSpawner.ResumeSongGameplay` (`self.NoteSpawnerRef `))
        (set `self.CurrentStep` 5)))
    (:`5`
      (`Widget.RemoveFromParent` (`self.TutorialWidget`)))))

(fn `UserConstructionScript`)