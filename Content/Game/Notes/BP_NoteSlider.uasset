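; BP_NoteSlider is a rhythm-game hold note that falls along Z each tick, with body and tail sized from its duration and fall speed.
; StartSlider sets timers that open the release window, force a late-release miss and periodically grant hold reward and healing.
; ReleaseSlider completes or fails the note by timing.
; Outcomes report score or miss to ThirdPersonCharacter, clear the lane's hold and destroy the actor.
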(event `ReleaseSlider`
  (if (`self.bSliderStarted`)
    (if (`self.CanReleaseSlider`)
      (`self.CompleteSlider`)
      (else
        (set `self.bSliderFailed` true)
        (set `self.WasHit` true)
        (bind _asthird_person_character (cast `/Game/Game/Character/Blueprints/ThirdPersonCharacter` (`GameplayStatics.GetPlayerCharacter` 0)))
        (`/Game/Game/Character/Blueprints/ThirdPersonCharacter.RegisterMiss` _asthird_person_character)
        (`/Game/Game/Character/Blueprints/ThirdPersonCharacter.ClearHoldingSlider` _asthird_person_character (`self.LaneIndex`))
        (`self.K2_DestroyActor`)))))

(event `LateReleaseMiss`
  (if (and (and (`self.bSliderStarted`) (not (`self.bSliderCompleted`))) (not (`self.bSliderFailed`)))
    _
    (else
      _))
  (set `self.bSliderFailed` true)
  (set `self.WasHit` true)
  (bind _asthird_person_character (cast `/Game/Game/Character/Blueprints/ThirdPersonCharacter` (`GameplayStatics.GetPlayerCharacter` 0)))
  (`/Game/Game/Character/Blueprints/ThirdPersonCharacter.returnOpacity` _asthird_person_character (`self.LaneIndex`))
  (`/Game/Game/Character/Blueprints/ThirdPersonCharacter.RegisterMiss` _asthird_person_character)
  (`/Game/Game/Character/Blueprints/ThirdPersonCharacter.ClearHoldingSlider` _asthird_person_character (`self.LaneIndex`))
  (`self.K2_DestroyActor`))

(event `CompleteSlider`
  (set `self.bSliderCompleted` true)
  (set `self.WasHit` true)
  (bind _asthird_person_character (cast `/Game/Game/Character/Blueprints/ThirdPersonCharacter` (`GameplayStatics.GetPlayerCharacter` 0)))
  (`/Game/Game/Character/Blueprints/ThirdPersonCharacter.AddScoreAndCombo` _asthird_person_character)
  (`/Game/Game/Character/Blueprints/ThirdPersonCharacter.ClearHoldingSlider` _asthird_person_character (`self.LaneIndex`))
  (`self.K2_DestroyActor`))

(event `StartSlider`
  (set `self.bSliderStarted` true)
  (set `self.WasHit` true)
  (set `self.CanReleaseSlider` false)
  (`KismetSystemLibrary.K2_SetTimerDelegate` (delegate `AllowSliderRelease`) (`KismetMathLibrary.FMax` (- (- (`self.EndTime`) (`self.HitTime`)) (`self.ReleaseWindow`)) 0.05))
  (`KismetSystemLibrary.K2_SetTimerDelegate` (delegate `LateReleaseMiss`) (`KismetMathLibrary.FMax` (+ (- (`self.EndTime`) (`self.HitTime`)) (`self.ReleaseWindow`)) 0.05))
  (`KismetSystemLibrary.K2_SetTimerDelegate` (delegate `GiveHoldReward`) 0.35 true))

(event `AllowSliderRelease`
  (set `self.CanReleaseSlider` true))

(event `GiveHoldReward`
  (if (and (and (`self.bSliderStarted`) (not (`self.bSliderCompleted`))) (not (`self.bSliderFailed`)))
    (bind _asthird_person_character (cast `/Game/Game/Character/Blueprints/ThirdPersonCharacter` (`GameplayStatics.GetPlayerCharacter` 0)))
    (`/Game/Game/Character/Blueprints/ThirdPersonCharacter.AddHoldReward` _asthird_person_character)
    (`/Game/Game/Character/Blueprints/ThirdPersonCharacter.healHP` _asthird_person_character)))

(event `self.ReceiveBeginPlay`
  (bind _output_get (set `self.SliderLength` (* (`self.FallSpeed`) (`KismetMathLibrary.FMax` (- (`self.EndTime`) (`self.HitTime`)) 0.1))))
  (`SceneComponent.SetRelativeScale3D` (`self.BodyMesh`) (`KismetMathLibrary.MakeVector` 0.6 0.3375 (/ _output_get 100.0)))
  (`SceneComponent.K2_SetRelativeLocation` (`self.BodyMesh`) (`KismetMathLibrary.MakeVector` 0.0 0.0 (/ _output_get 2.0)) false false)
  (`SceneComponent.K2_SetRelativeLocation` (`self.TailMesh`) (`KismetMathLibrary.MakeVector` 0.0 -134.0 _output_get) false false))

(event `self.ReceiveTick`
  (params (DeltaSeconds :type "Float (single-precision)"))
  (`self.K2_SetActorLocation` (`KismetMathLibrary.MakeVector` (.x (`self.K2_GetActorLocation`)) (.y (`self.K2_GetActorLocation`)) (- (.z (`self.K2_GetActorLocation`)) (* DeltaSeconds (`self.FallSpeed`))))))

(fn `UserConstructionScript`)