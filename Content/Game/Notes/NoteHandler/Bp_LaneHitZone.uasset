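; Lane hit zone for a three-lane note game that tells the player which note is currently hittable.
; On overlap, it stores the BP_NoteTEST in the ThirdPersonCharacter's active-note slot chosen by LaneIndex.
; When an unhit note leaves, it checks the character's own WasHit flag: true clears that lane's slot, false deducts score and prints it without clearing.
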(event `self.ReceiveActorBeginOverlap`
  (params (OtherActor :type "Actor Object Reference"))
  (bind _asbp_note_test (cast `/Game/Game/Notes/BP_NoteTEST` OtherActor))
  (bind _asthird_person_character (cast `/Game/Game/Character/Blueprints/ThirdPersonCharacter` (`GameplayStatics.GetPlayerCharacter` 0)))
  (switch `int` (`self.LaneIndex`)
    (:`0`
      (set `/Game/Game/Character/Blueprints/ThirdPersonCharacter.ActiveNoteLane0` _asbp_note_test _asthird_person_character))
    (:`1`
      (set `/Game/Game/Character/Blueprints/ThirdPersonCharacter.ActiveNoteLane1` _asbp_note_test _asthird_person_character))
    (:`2`
      (set `/Game/Game/Character/Blueprints/ThirdPersonCharacter.ActiveNoteLane2` _asbp_note_test _asthird_person_character))))

(event `self.ReceiveActorEndOverlap`
  (params (OtherActor :type "Actor Object Reference"))
  (bind _asbp_note_test (cast `/Game/Game/Notes/BP_NoteTEST` OtherActor))
  (if (not (`/Game/Game/Notes/BP_NoteTEST.WasHit` _asbp_note_test))
    (bind _asthird_person_character (cast `/Game/Game/Character/Blueprints/ThirdPersonCharacter` (`GameplayStatics.GetPlayerCharacter` 0)))
    (if (`/Game/Game/Character/Blueprints/ThirdPersonCharacter.WasHit` _asthird_person_character)
      (switch `int` (`self.LaneIndex`)
        (:`0`
          (set `/Game/Game/Character/Blueprints/ThirdPersonCharacter.ActiveNoteLane0` null _asthird_person_character))
        (:`1`
          (set `/Game/Game/Character/Blueprints/ThirdPersonCharacter.ActiveNoteLane1` null _asthird_person_character))
        (:`2`
          (set `/Game/Game/Character/Blueprints/ThirdPersonCharacter.ActiveNoteLane2` null _asthird_person_character)))
      (else
        (bind _output_get (set `/Game/Game/Character/Blueprints/ThirdPersonCharacter.Score` (- (`/Game/Game/Character/Blueprints/ThirdPersonCharacter.Score` _asthird_person_character) 10) _asthird_person_character))
        (`KismetSystemLibrary.PrintString` (`KismetStringLibrary.Conv_IntToString` _output_get))))))

(fn `UserConstructionScript`)