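; Rhythm-game spawner actor that plays a song and spawns falling-note actors for three lanes from a chart Data Table.
; BeginPlay loads the chart rows into an array, then starts the audio and song timer.
; Tick accumulates delta time, spawning at most one note per frame, TravelTime ahead of its HitTime.
; Notes spawn above their lane cube and receive the lane index, though lane 0's spawn has no class set.
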(event `StartSong`
  (set `self.NextNoteIndex` 0)
  (set `self.SongTime` 0.0)
  (set `self.SongStarted` true)
  (`GameplayStatics.PlaySound2D` (`self.SongAudio`) 1.0 1.0 0.0 null null))

(event `self.ReceiveBeginPlay`
  (`KismetArrayLibrary.Array_Clear` (`self.ParsedNotes`))
  (bind _outrownames (`DataTableFunctionLibrary.GetDataTableRowNames` (`self.NoteChart`)))
  (for _array_element _outrownames
    (bind _returnvalue (`|GetDataTableRow` (`self.NoteChart`) _array_element)
      (:`then`
        (`KismetArrayLibrary.Array_Add` (`self.ParsedNotes`) _returnvalue))))
  (set `self.NextNoteIndex` 0)
  (set `self.SongTime` 0.0)
  (set `self.SongStarted` false)
  (`KismetSystemLibrary.PrintString` (`KismetTextLibrary.Conv_TextToString` (`KismetTextLibrary.Conv_Int64ToText` 0 false true (`KismetArrayLibrary.Array_Length` (`self.ParsedNotes`)))))
  (`self.StartSong`))

(event `self.ReceiveTick`
  (params (DeltaSeconds :type "Float (single-precision)"))
  (bind (_hittime _lane) (break `/Game/Game/Notes/NoteHandler/ST_NoteData` (`|GetArrayItem` (`self.ParsedNotes`) (`self.NextNoteIndex`))))
  (if (`self.SongStarted`)
    (set `self.SongTime` (+ (`self.SongTime`) DeltaSeconds))
    (if (< (`self.NextNoteIndex`) (`KismetArrayLibrary.Array_Length` (`self.ParsedNotes`)))
      (if (>= (`self.SongTime`) (- _hittime (`self.TravelTime`)))
        (`self.SpawnNoteForLane` _lane)
        (set `self.NextNoteIndex` (+ (`self.NextNoteIndex`) 1))))))

(fn `SpawnNoteForLane`
  (params (Lane :type Integer))
  (switch `int` Lane
    (:`0`
      (bind _returnvalue (`|SpawnActorFromClass` "/Game/Game/Notes/BP_NoteTEST.BP_NoteTEST_C" (`KismetMathLibrary.MakeTransform` (+ (`self.K2_GetActorLocation` (`self.LaneCube0`)) (`KismetMathLibrary.MakeVector` 0.0 0.0 (`self.SpawnHeight`)))) "Undefined" "OverrideRootScale" null null))
      (bind _asbp_note_test (cast `/Game/Game/Notes/BP_NoteTEST` _returnvalue))
      (set `/Game/Game/Notes/BP_NoteTEST.LaneIndex` (`local.Lane`) _asbp_note_test))
    (:`1`
      (bind _returnvalue_2 (`|SpawnActorFromClass` "/Game/Game/Notes/BP_NoteTEST.BP_NoteTEST_C" (`KismetMathLibrary.MakeTransform` (+ (`self.K2_GetActorLocation` (`self.LaneCube1`)) (`KismetMathLibrary.MakeVector` 0.0 0.0 (`self.SpawnHeight`)))) "Undefined" "OverrideRootScale" null null))
      (bind _asbp_note_test_2 (cast `/Game/Game/Notes/BP_NoteTEST` _returnvalue_2))
      (set `/Game/Game/Notes/BP_NoteTEST.LaneIndex` (`local.Lane`) _asbp_note_test_2))
    (:`2`
      (bind _returnvalue_3 (`|SpawnActorFromClass` "/Game/Game/Notes/BP_NoteTEST.BP_NoteTEST_C" (`KismetMathLibrary.MakeTransform` (+ (`self.K2_GetActorLocation` (`self.LaneCube2`)) (`KismetMathLibrary.MakeVector` 0.0 0.0 (`self.SpawnHeight`)))) "Undefined" "OverrideRootScale" null null))
      (bind _asbp_note_test_3 (cast `/Game/Game/Notes/BP_NoteTEST` _returnvalue_3))
      (set `/Game/Game/Notes/BP_NoteTEST.LaneIndex` (`local.Lane`) _asbp_note_test_3))))

(fn `UserConstructionScript`)